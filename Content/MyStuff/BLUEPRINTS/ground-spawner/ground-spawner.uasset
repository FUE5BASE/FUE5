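; Ground spawner actor that sizes the level's ground to fit entity positions read from a JSON file.
; Its Construction Script parses the file at Path and scans the "entities" array for the largest x and y.
; Those extents scale the first Landscape found in the level and the actor's Static mesh plane.
; The plane gets a dynamic material instance whose U and V tiling follow the same extents.
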(event EventBeginPlay)

(event Collision|EventActorBeginOverlap
  (params (OtherActor :type Actor%20Object%20Reference)))

(event EventTick
  (params (DeltaSeconds :type Float%20%28single-precision%29)))

(fn ConstructionScript
  (bind _returnvalue (Math|Float|MakeLiteralFloat 1.0))
  (bind _returnvalue_2 (Math|Float|MakeLiteralFloat 0.12))
  (bind _returnvalue_3 (Math|Float|MakeLiteralFloat 3.7))
  (bind _static (Variables|Default|Getstatic))
  ;[1 1 1] json parser
  (Utilities|FlowControl|Sequence
    (:then_0
      (bind _outjsonobject (Class|JsonBlueprintFunctionLibrary|FromFile (Utilities|Struct|MakeFilePath (Variables|Default|Getpath))))
      (Utilities|FlowControl|Sequence
        (:then_0
          (bind _outvalue (|GetJsonField _outjsonobject "entities"))
          (for _array_element _outvalue
            ;[1 1 1] coordinate translate
            (bind _outvalue_2 (|GetJsonField _array_element "x"))
            (Utilities|FlowControl|Sequence
              (:then_1
                (Math|Float|CompareFloat _outvalue_2 (Variables|Default|Getx_end)
                  (:>
                    (Variables|Default|Setx_end _outvalue_2))))
              (:then_2
                (bind _outvalue_3 (|GetJsonField _array_element "y"))
                (Utilities|FlowControl|Sequence
                  (:then_1
                    (Math|Float|CompareFloat _outvalue_3 (Variables|Default|Gety_end)
                      (:>
                        (Variables|Default|Sety_end _outvalue_3))))))))
          ;[1 1 1] landscape scale
          (bind _outactors (Actor|GetAllActorsOfClass "/Script/Landscape.Landscape"))
          (Transformation|SetActorScale3D (Utilities|Array|Get(acopy) _outactors) (Math|Vector|MakeVector (* (Variables|Default|Getx_end) _returnvalue_3) (* (Variables|Default|Gety_end) _returnvalue_3) (* (Variables|Default|Gety_end) _returnvalue_3)))
          ;[1 1 1] make plane
          (bind _returnvalue_4 (Rendering|Material|CreateDynamicMaterialInstance (Variables|Default|Getsurface-material) "" "None" :!class /Script/Engine.KismetMaterialLibrary))
          (Rendering|Material|SetScalarParameterValue _returnvalue_4 "UTiling" (* (Variables|Default|Getx_end) _returnvalue_2) :!class /Script/Engine.MaterialInstanceDynamic)
          (Rendering|Material|SetScalarParameterValue _returnvalue_4 "VTiling" (* (Variables|Default|Gety_end) _returnvalue_2) :!class /Script/Engine.MaterialInstanceDynamic)
          (Rendering|Material|SetMaterial _static 0 _returnvalue_4)
          (Transformation|SetRelativeScale3D _static (Math|Vector|MakeVector (* (Variables|Default|Getx_end) _returnvalue) (* (Variables|Default|Gety_end) _returnvalue) 1.0)))))))