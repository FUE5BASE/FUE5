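; Structure system that, in its construction script, builds the level's entities and wires from the exported data of its parent json-loader actor.
; Entity names resolve through a cascade of class maps into child actors, which receive their variant through _HasVariants.
; Known missing entities become placeholder cubes, while two special names become a hand-placed sign and rocket.
; Wires are child actors rotated toward their target and stretched along X to span each connection.
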(fn ConstructionScript
  (bind _asjson_loader (Utilities|Casting|CastTojson-loader (Actor|GetParentActor)))
  (Utilities|FlowControl|Sequence
    (:then_0
      ;[1 1 1] Spawn entities
      (for _array_element (Variables|/Game/MyStuff/BLUEPRINTS/json-loader/json-loader.json-loader_C|GetexportedEntities _asjson_loader)
        ;;[1 1 1] choose entity and spawn
        (bind _returnvalue (AddComponent|AddChildActorComponent false (Math|Transform|MakeTransform (Variables|/Game/MyStuff/BLUEPRINTS/json-loader/ExportedEntity.ExportedEntity_C|Getlocation _array_element) (* (Math|Rotator|MakeRotator 0.0 0.0 (Math|Conversions|ToFloat(Integer) (Variables|/Game/MyStuff/BLUEPRINTS/json-loader/ExportedEntity.ExportedEntity_C|Getdirection _array_element))) 45.0))))
        (if (.ReturnValue (Utilities|Map|Find (Variables|Default|Getvariants) (Variables|/Game/MyStuff/BLUEPRINTS/json-loader/ExportedEntity.ExportedEntity_C|Getname _array_element)))
          (ChildActorComponent|SetChildActorClass _returnvalue (.Value (Utilities|Map|Find (Variables|Default|Getvariants) (Variables|/Game/MyStuff/BLUEPRINTS/json-loader/ExportedEntity.ExportedEntity_C|Getname _array_element))))
          (bind _as_has_variants (Utilities|Casting|CastTo_HasVariants (Variables|/Script/Engine.ChildActorComponent|GetChildActor _returnvalue) :!label _label)
            (:then
              (Default|SetVariant _as_has_variants (Variables|/Game/MyStuff/BLUEPRINTS/json-loader/ExportedEntity.ExportedEntity_C|Getvariant _array_element)))
            (:CastFailed
              _))
          (Variables|/Game/MyStuff/BLUEPRINTS/json-loader/ExportedEntity.ExportedEntity_C|Setactor _array_element (Variables|/Script/Engine.ChildActorComponent|GetChildActor _returnvalue) :!label _label_2)
          (elif (.ReturnValue (Utilities|Map|Find (Variables|Default|Getstructures) (Variables|/Game/MyStuff/BLUEPRINTS/json-loader/ExportedEntity.ExportedEntity_C|Getname _array_element)))
            (ChildActorComponent|SetChildActorClass _returnvalue (.Value (Utilities|Map|Find (Variables|Default|Getstructures) (Variables|/Game/MyStuff/BLUEPRINTS/json-loader/ExportedEntity.ExportedEntity_C|Getname _array_element))))
            (goto _label)
            (elif (.ReturnValue (Utilities|Map|Find (Variables|Default|Getpower) (Variables|/Game/MyStuff/BLUEPRINTS/json-loader/ExportedEntity.ExportedEntity_C|Getname _array_element)))
              (ChildActorComponent|SetChildActorClass _returnvalue (.Value (Utilities|Map|Find (Variables|Default|Getpower) (Variables|/Game/MyStuff/BLUEPRINTS/json-loader/ExportedEntity.ExportedEntity_C|Getname _array_element))))
              (goto _label)
              (elif (.ReturnValue (Utilities|Map|Find (Variables|Default|Getfoliage) (Variables|/Game/MyStuff/BLUEPRINTS/json-loader/ExportedEntity.ExportedEntity_C|Getname _array_element)))
                (ChildActorComponent|SetChildActorClass _returnvalue (.Value (Utilities|Map|Find (Variables|Default|Getfoliage) (Variables|/Game/MyStuff/BLUEPRINTS/json-loader/ExportedEntity.ExportedEntity_C|Getname _array_element))))
                (goto _label)
                (elif (.ReturnValue (Utilities|Map|Find (Variables|Default|Getmissing) (Variables|/Game/MyStuff/BLUEPRINTS/json-loader/ExportedEntity.ExportedEntity_C|Getname _array_element)))
                  (bind _returnvalue_2 (AddComponent|AddStaticMeshComponent false (Math|Transform|MakeTransform (Variables|/Game/MyStuff/BLUEPRINTS/json-loader/ExportedEntity.ExportedEntity_C|Getlocation _array_element) (* (Math|Rotator|MakeRotator 0.0 0.0 (Math|Conversions|ToFloat(Integer) (Variables|/Game/MyStuff/BLUEPRINTS/json-loader/ExportedEntity.ExportedEntity_C|Getdirection _array_element))) 45.0) (* (Math|Vector|MakeVector (Variables|/Game/MyStuff/BLUEPRINTS/json-loader/ExportedEntity.ExportedEntity_C|Getwidth _array_element) (Variables|/Game/MyStuff/BLUEPRINTS/json-loader/ExportedEntity.ExportedEntity_C|Getheight _array_element) 1.0) "2.000000,2.000000,2.000000"))))
                  (Components|StaticMesh|SetStaticMesh _returnvalue_2 "/Game/StarterContent/Shapes/Shape_Cube.Shape_Cube")
                  (Rendering|Material|SetMaterial _returnvalue_2 0 "/Game/MyStuff/BLUEPRINTS/structure-system/missing-entity.missing-entity")
                  (goto _label_2)
                  (elif (Utilities|Enum|Equal(Enum) (Variables|/Game/MyStuff/BLUEPRINTS/json-loader/ExportedEntity.ExportedEntity_C|Getname _array_element) (Utilities|String|MakeLiteralString "heat-interface"))
                    (bind _returnvalue_3 (AddComponent|AddChildActorComponent false (Math|Transform|MakeTransform "11800.000000,9200.000000,0.000000")))
                    (ChildActorComponent|SetChildActorClass _returnvalue_3 "/Game/MyStuff/LEVELS/LOAD/ENTITIES/sign1/bp/sign1_1.sign1_1_C")
                    (goto _label_2)
                    (elif (Utilities|Enum|Equal(Enum) (Variables|/Game/MyStuff/BLUEPRINTS/json-loader/ExportedEntity.ExportedEntity_C|Getname _array_element) (Utilities|String|MakeLiteralString "infinity-chest"))
                      (bind _returnvalue_4 (AddComponent|AddChildActorComponent false (Math|Transform|MakeTransform "14923.419677,5089.392331,533.000000" "0.000000,-65.330562,90.000000" "1.931422,1.931422,1.931422")))
                      (ChildActorComponent|SetChildActorClass _returnvalue_4 "/Game/MyStuff/ENTITIES/VEHICLES/rocket/bp/rocket.rocket_C")
                      (goto _label_2))))))))))
    (:then_1
      ;[1 1 1] wires
      (for _array_element_2 (Variables|/Game/MyStuff/BLUEPRINTS/json-loader/json-loader.json-loader_C|GetwireConnections _asjson_loader)
        (bind _returnvalue_5 (AddComponent|AddChildActorComponent false (Math|Conversions|ToTransform(Vector) (* (.start (Utilities|Struct|BreakWireConnection _array_element_2)) "200.000000,200.000000,200.000000"))))
        (Transformation|SetRelativeRotation _returnvalue_5 (Math|Rotator|FindLookatRotation (* (.start (Utilities|Struct|BreakWireConnection _array_element_2)) "200.000000,200.000000,200.000000") (* (.target (Utilities|Struct|BreakWireConnection _array_element_2)) "200.000000,200.000000,200.000000")) false false)
        (Transformation|SetWorldScale3D _returnvalue_5 (Math|Vector|MakeVector (/ (Math|Vector|VectorLength (- (* (.start (Utilities|Struct|BreakWireConnection _array_element_2)) "200.000000,200.000000,200.000000") (* (.target (Utilities|Struct|BreakWireConnection _array_element_2)) "200.000000,200.000000,200.000000"))) 4e+02) 1.0 1.0))))))