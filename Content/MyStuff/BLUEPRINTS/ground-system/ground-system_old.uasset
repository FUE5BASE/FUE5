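; Legacy ground-system actor for sizing the level floor to parent json-loader bounds; its construction script is empty and all logic is disconnected.
; One unused chain scales and positions a static ground plane with tiled dynamic material, moves the actor and scales the first Landscape.
; Another builds a dynamic-mesh box from bounds width, then boolean-subtracts cylinders at each Rocketsilo to cut holes.
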(fn ConstructionScript)