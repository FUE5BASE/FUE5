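; Ground actor for a level built by its parent json-loader, sized to the loader's bounds.
; Its construction script generates a Geometry Script box with a dynamic material whose tiling scales with those bounds.
; Boolean subtraction cuts a cylindrical hole at each Rocketsilo.
; If a Landscape exists, it repositions itself, scales the first Landscape to the bounds and unhides it in game when exported entities include a linked-belt.
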(fn ConstructionScript
  (bind _returnvalue (Math|Float|MakeLiteralFloat 0.12))
  (bind _asjson_loader (Utilities|Casting|CastTojson-loader (Actor|GetParentActor)))
  (Utilities|FlowControl|Sequence
    (:then_0
      ;[1 1 1] GeometryScript ground
      ;;[1 1 1] material
      (bind _returnvalue_2 (Rendering|Material|CreateDynamicMaterialInstance "/Game/MyStuff/BLUEPRINTS/ground-system/ground-material/ground-material.ground-material" "" "None" :!class /Script/Engine.KismetMaterialLibrary))
      (Rendering|Material|SetScalarParameterValue _returnvalue_2 "UTiling" (* (.width (Utilities|Struct|BreakBounds (Variables|/Game/MyStuff/BLUEPRINTS/json-loader/json-loader.json-loader_C|Getbounds _asjson_loader))) _returnvalue) :!class /Script/Engine.MaterialInstanceDynamic)
      (Rendering|Material|SetScalarParameterValue _returnvalue_2 "VTiling" (* _returnvalue (.height (Utilities|Struct|BreakBounds (Variables|/Game/MyStuff/BLUEPRINTS/json-loader/json-loader.json-loader_C|Getbounds _asjson_loader)))) :!class /Script/Engine.MaterialInstanceDynamic))
    (:then_1
      (Utilities|FlowControl|Sequence
        (:then_0
          (bind _returnvalue_3 (AddComponent|AddDynamicMeshComponent false))
          (GeometryScript|Scene|SetComponentMaterialList _returnvalue_3 (Utilities|Array|MakeArray _returnvalue_2) 0)
          (bind _returnvalue_4 (DynamicMeshComponent|GetDynamicMesh _returnvalue_3))
          (bind _returnvalue_5 (DynamicMesh|Reset _returnvalue_4))
          (bind _returnvalue_6 (Class|GeometryScriptLibraryMeshPrimitiveFunctions|AppendBox :TargetMesh _returnvalue_5 :Transform (Math|Transform|MakeTransform (* (Math|Vector|MakeVector (.width (Utilities|Struct|BreakBounds (Variables|/Game/MyStuff/BLUEPRINTS/json-loader/json-loader.json-loader_C|Getbounds _asjson_loader))) (.height (Utilities|Struct|BreakBounds (Variables|/Game/MyStuff/BLUEPRINTS/json-loader/json-loader.json-loader_C|Getbounds _asjson_loader))) 0.0) "100.000000,100.000000,1.000000")) :DimensionX (* (.width (Utilities|Struct|BreakBounds (Variables|/Game/MyStuff/BLUEPRINTS/json-loader/json-loader.json-loader_C|Getbounds _asjson_loader))) 2e+02) :DimensionY (* (.height (Utilities|Struct|BreakBounds (Variables|/Game/MyStuff/BLUEPRINTS/json-loader/json-loader.json-loader_C|Getbounds _asjson_loader))) 2e+02) :DimensionZ 0.1 :Debug 0)))
        (:then_1
          ;;[1 1 1] boolean
          (bind _outactors (Actor|GetAllActorsOfClass "/Game/MyStuff/ENTITIES/STRUCTURES/rocket-silo/bp/rocket-silo.rocket-silo_C"))
          (for (_ _array_index) _outactors
            (bind _returnvalue_7 (DynamicMeshActor|AllocateComputeMesh))
            (bind _returnvalue_8 (GeometryScript|Primitives|AppendCylinder :TargetMesh _returnvalue_7 :Transform (Math|Transform|MakeTransform (Transformation|GetActorLocation (Utilities|Array|Get(acopy) _outactors _array_index))) :Radius 7e+02 :Height 5e+02 :RadialSteps 20 :Origin "Center" :Debug 0))
            (GeometryScript|Booleans|ApplyMeshBoolean :TargetMesh _returnvalue_6 :ToolMesh _returnvalue_8 :Operation "Subtract" :Debug 0)))))
    (:then_2
      ;[1 1 1] landscape scale
      (bind _outactors_2 (Actor|GetAllActorsOfClass "/Script/Landscape.Landscape"))
      (if (Utilities|Array|IsNotEmpty _outactors_2)
        (Transformation|SetActorLocation (* (Math|Vector|MakeVector (.x (Utilities|Struct|BreakBounds (Variables|/Game/MyStuff/BLUEPRINTS/json-loader/json-loader.json-loader_C|Getbounds _asjson_loader))) (.y (Utilities|Struct|BreakBounds (Variables|/Game/MyStuff/BLUEPRINTS/json-loader/json-loader.json-loader_C|Getbounds _asjson_loader))) 0.0) "200.000000,200.000000,1.000000") false true)
        (Transformation|SetActorScale3D (Utilities|Array|Get(acopy) _outactors_2) (* (Math|Vector|MakeVector (.width (Utilities|Struct|BreakBounds (Variables|/Game/MyStuff/BLUEPRINTS/json-loader/json-loader.json-loader_C|Getbounds _asjson_loader))) (.height (Utilities|Struct|BreakBounds (Variables|/Game/MyStuff/BLUEPRINTS/json-loader/json-loader.json-loader_C|Getbounds _asjson_loader))) 1.0) "3.571000,3.571000,1.000000"))
        (bind _array_element (Utilities|Array|ForEachLoopwithBreak (Variables|/Game/MyStuff/BLUEPRINTS/json-loader/json-loader.json-loader_C|Getexported-entities _asjson_loader) :!label _label)
          (:LoopBody
            (if (Utilities|Enum|Equal(Enum) (Variables|/Game/MyStuff/BLUEPRINTS/json-loader/ExportedEntity.ExportedEntity_C|Getname _array_element) (Utilities|String|MakeLiteralString "linked-belt"))
              (Rendering|SetActorHiddenInGame (Utilities|Array|Get(acopy) _outactors_2) false)
              (goto _label Break))))))))