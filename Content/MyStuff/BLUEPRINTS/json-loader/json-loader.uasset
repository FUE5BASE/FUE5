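; Loader actor that imports a JSON export of a factory layout and spawns the systems for it at construction time.
; The construction script reads a configurable path, with a project default, into bounds, entities, wire connections, train paths, belt paths and logistic systems.
; Entities parse first with grid positions scaled to world units, so later parsers resolve indices against that array.
; It then adds optional structure, rail, belt, logistic and ground child actors.
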(event EventBeginPlay)

(event Collision|EventActorBeginOverlap
  (params (OtherActor :type Actor%20Object%20Reference)))

(event EventTick
  (params (DeltaSeconds :type Float%20%28single-precision%29)))

(fn ConstructionScript
  (bind _returnvalue (Class|KismetSystemLibrary|GetProjectDirectory))
  (bind _json_file_path (Variables|USERSETTINGS|GetJSON%20file%20path))
  (if (Variables|USERSETTINGS|GetRefresh%20Base)
    (Variables|USERSETTINGS|SetRefresh%20Base false))
  (bind _outjsonobject (Class|JsonBlueprintFunctionLibrary|FromFile (Utilities|Struct|MakeFilePath (Utilities|String|SelectString (Class|BlueprintPathsLibrary|Combine (Utilities|Array|MakeArray _returnvalue "Content" "MyStuff" "JSON" "exported-entities.json")) (Utilities|String|SelectString (Class|BlueprintPathsLibrary|Combine (Utilities|Array|MakeArray _returnvalue _json_file_path)) _json_file_path (Class|BlueprintPathsLibrary|IsRelative _json_file_path)) (Utilities|Array|IsEmpty _json_file_path)))))
  (Utilities|FlowControl|Sequence
    (:then_0
      ;[1 1 1] Load JSON
      (bind _outvalue (|GetJsonField _outjsonobject "bounds"))
      (bind _bounds (CallFunction|ParseBounds _outvalue))
      (Variables|Default|Setbounds _bounds))
    (:then_1
      (bind _outvalue_2 (|GetJsonField _outjsonobject "entities"))
      (for _array_element _outvalue_2
        (bind _returnvalue_2 (CallFunction|ParseExportedEntity _array_element))
        (Utilities|Array|Add (Variables|Default|Getexported-entities) _returnvalue_2)))
    (:then_2
      (bind _outvalue_3 (|GetJsonField _outjsonobject "wire_connections"))
      (for _array_element_2 _outvalue_3
        (bind _result (CallFunction|ParseWireConnection _array_element_2))
        (Utilities|Array|Add (Variables|Default|Getwire-connections) _result)))
    (:then_3
      (bind _outvalue_4 (|GetJsonField _outjsonobject "train_paths"))
      (for _array_element_3 _outvalue_4
        (bind _result_2 (CallFunction|ParseTrainPath _array_element_3))
        (Utilities|Array|Add (Variables|Default|Gettrain-paths) _result_2)))
    (:then_4
      (bind _outvalue_5 (|GetJsonField _outjsonobject "belt_paths"))
      (for _array_element_4 _outvalue_5
        (bind _result_3 (CallFunction|ParseBeltPath _array_element_4))
        (Utilities|Array|Add (Variables|Default|Getbelt-paths) _result_3)))
    (:then_5
      (bind _outvalue_6 (|GetJsonField _outjsonobject "logistic_systems"))
      (for _array_element_5 _outvalue_6
        (bind _result_4 (CallFunction|ParseLogisticSystem _array_element_5))
        (Utilities|Array|Add (Variables|Default|Getlogistic-systems) _result_4)))
    (:then_6
      ;[1 1 1] Spawn systems
      (Utilities|FlowControl|Sequence
        (:then_0
          (if (Variables|CORESYSTEMS|GetStructure-system)
            (bind _returnvalue_3 (AddComponent|AddChildActorComponent false))
            (ChildActorComponent|SetChildActorClass _returnvalue_3 "/Game/MyStuff/BLUEPRINTS/structure-system/structure-system.structure-system_C")))
        (:then_1
          (if (Variables|CORESYSTEMS|GetRail-system)
            (bind _returnvalue_4 (AddComponent|AddChildActorComponent false))
            (ChildActorComponent|SetChildActorClass _returnvalue_4 "/Game/MyStuff/BLUEPRINTS/rail-system/rail-system.rail-system_C")))
        (:then_2
          (if (Variables|CORESYSTEMS|GetBelt-system)
            (bind _returnvalue_5 (AddComponent|AddChildActorComponent false))
            (ChildActorComponent|SetChildActorClass _returnvalue_5 "/Game/MyStuff/BLUEPRINTS/belt-system/belt-system.belt-system_C")))
        (:then_3
          (if (Variables|CORESYSTEMS|GetLogistic-system)
            (bind _returnvalue_6 (AddComponent|AddChildActorComponent false))
            (ChildActorComponent|SetChildActorClass _returnvalue_6 "/Game/MyStuff/BLUEPRINTS/logistic-system/logistic-system.logistic-system_C")))
        (:then_4
          (if (Variables|CORESYSTEMS|GetGround-system)
            (bind _returnvalue_7 (AddComponent|AddChildActorComponent false))
            (ChildActorComponent|SetChildActorClass _returnvalue_7 "/Game/MyStuff/BLUEPRINTS/ground-system/ground-system-dynamic.ground-system-dynamic_C")))))))

(fn ParseExportedEntity
  (params (JsonObject :type Json%20Object%20Wrapper%20Structure%20%28by%20ref%29))
  (bind _outvalue (|GetJsonField JsonObject "name"))
  (bind _outvalue_2 (|GetJsonField JsonObject "x"))
  (bind _outvalue_3 (|GetJsonField JsonObject "y"))
  (bind _outvalue_4 (|GetJsonField JsonObject "direction"))
  (bind _outvalue_5 (|GetJsonField JsonObject "width"))
  (bind _outvalue_6 (|GetJsonField JsonObject "height"))
  (bind _value (Utilities|GetFieldChecked JsonObject "back_mover" false))
  (bind _value_2 (Utilities|GetFieldChecked JsonObject "operation"))
  (bind _value_3 (Utilities|GetFieldChecked JsonObject "variant"))
  (bind _returnvalue (Game|ConstructObjectfromClass "/Game/MyStuff/BLUEPRINTS/json-loader/ExportedEntity.ExportedEntity_C" _outvalue _outvalue_2 _outvalue_3 _outvalue_4 (* (Math|Vector|MakeVector _outvalue_2 _outvalue_3 0.0) "200.000000,200.000000,200.000000") _outvalue_5 _outvalue_6 _value _value_2 _value_3 0))
  (return _returnvalue))

(fn ParseWireConnection
  (params (JsonObject :type Json%20Object%20Wrapper%20Structure%20%28by%20ref%29))
  (Utilities|FlowControl|Sequence
    (:then_0
      (bind _outvalue (|GetJsonField JsonObject "start"))
      (bind _outvalue_2 (|GetJsonField _outvalue "x"))
      (bind _outvalue_3 (|GetJsonField _outvalue "y"))
      (bind _outvalue_4 (|GetJsonField _outvalue "z")))
    (:then_1
      (bind _outvalue_5 (|GetJsonField JsonObject "target"))
      (bind _outvalue_6 (|GetJsonField _outvalue_5 "x"))
      (bind _outvalue_7 (|GetJsonField _outvalue_5 "y"))
      (bind _outvalue_8 (|GetJsonField _outvalue_5 "z")))
    (:then_2
      (return (Utilities|Struct|MakeWireConnection (Math|Vector|MakeVector _outvalue_2 _outvalue_3 _outvalue_4) (Math|Vector|MakeVector _outvalue_6 _outvalue_7 _outvalue_8))))))

(fn ParseTrainPath
  (params (JsonObject :type Json%20Object%20Wrapper%20Structure%20%28by%20ref%29))
  (Utilities|FlowControl|Sequence
    (:then_0
      (bind _outvalue (|GetJsonField JsonObject "carriages"))
      (bind _arrayout (Utilities|SetTempArray (Utilities|Array|MakeArray))
        (:ExecOut
          (for _array_element _outvalue
            (Utilities|Array|Add _arrayout (Utilities|Array|Get(acopy) (Variables|Default|Getexported-entities) _array_element))))))
    (:then_1
      (bind _outvalue_2 (|GetJsonField JsonObject "path"))
      (bind _arrayout_2 (Utilities|SetTempArray (Utilities|Array|MakeArray))
        (:ExecOut
          (for _array_element_2 _outvalue_2
            (bind _outvalue_3 (|GetJsonField _array_element_2 "index"))
            (bind _outvalue_4 (|GetJsonField _array_element_2 "invert_spline"))
            (Utilities|Array|Add _arrayout_2 (Utilities|Struct|MakeTrainPathSegment (Utilities|Array|Get(acopy) (Variables|Default|Getexported-entities) _outvalue_3) _outvalue_4))))))
    (:then_2
      (return (Utilities|Struct|MakeTrainPath _arrayout _arrayout_2)))))

(fn ParseBeltPath
  (params (JsonObject :type Json%20Object%20Wrapper%20Structure%20%28by%20ref%29))
  (Utilities|FlowControl|Sequence
    (:then_0
      (bind _outvalue (|GetJsonField JsonObject "path"))
      (bind _arrayout (Utilities|SetTempArray (Utilities|Array|MakeArray))
        (:ExecOut
          (for _array_element _outvalue
            (Utilities|Array|Add _arrayout (Utilities|Array|Get(acopy) (Variables|Default|Getexported-entities) _array_element))))))
    (:then_1
      (bind _outvalue_2 (|GetJsonField JsonObject "items_lane_r"))
      (bind _arrayout_2 (Utilities|SetTempArray (Utilities|Array|MakeArray))
        (:ExecOut
          (for _array_element_2 _outvalue_2
            (Utilities|Array|Add _arrayout_2 _array_element_2)))))
    (:then_2
      (bind _outvalue_3 (|GetJsonField JsonObject "items_lane_l"))
      (bind _arrayout_3 (Utilities|SetTempArray (Utilities|Array|MakeArray))
        (:ExecOut
          (for _array_element_3 _outvalue_3
            (Utilities|Array|Add _arrayout_3 _array_element_3)))))
    (:then_3
      (return (Utilities|Struct|MakeBeltPath _arrayout _arrayout_2 _arrayout_3)))))

(fn ParseLogisticSystem
  (params (JsonObject :type Json%20Object%20Wrapper%20Structure))
  (Utilities|FlowControl|Sequence
    (:then_0
      (bind _outvalue (|GetJsonField JsonObject "roboports"))
      (bind _arrayout (Utilities|SetTempArray (Utilities|Array|MakeArray))
        (:ExecOut
          (for _array_element _outvalue
            (Utilities|Array|Add _arrayout (Utilities|Array|Get(acopy) (Variables|Default|Getexported-entities) _array_element))))))
    (:then_1
      (bind _outvalue_2 (|GetJsonField JsonObject "chests"))
      (bind _arrayout_2 (Utilities|SetTempArray (Utilities|Array|MakeArray))
        (:ExecOut
          (for _array_element_2 _outvalue_2
            (Utilities|Array|Add _arrayout_2 (Utilities|Array|Get(acopy) (Variables|Default|Getexported-entities) _array_element_2))))))
    (:then_2
      (return (Utilities|Struct|MakeLogisticSystem _arrayout _arrayout_2)))))

(fn ParseBounds
  (params (JsonObject :type Json%20Object%20Wrapper%20Structure%20%28by%20ref%29))
  (bind _outvalue (|GetJsonField JsonObject "x"))
  (bind _outvalue_2 (|GetJsonField JsonObject "y"))
  (bind _outvalue_3 (|GetJsonField JsonObject "width"))
  (bind _outvalue_4 (|GetJsonField JsonObject "height"))
  (return (Utilities|Struct|MakeBounds _outvalue _outvalue_2 _outvalue_3 _outvalue_4)))