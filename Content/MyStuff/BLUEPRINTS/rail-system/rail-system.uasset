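; Rail system actor that builds train tracks from the parent json-loader's TrainPaths and runs carriages along them.
; Construction stitches rotated template rail splines into one spline per path, closing near-touching ends, then spawns carriage child actors with optional 180-degree flips.
; Tick derives eased, wrapping distance from game time and a random start delay, spacing carriages by index along the spline.
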(event EventTick
  (params (DeltaSeconds :type Float%20%28single-precision%29))
  (for _array_element (Variables|Default|GettrainSplines)
    (for (_array_element_2 _array_index) (.carriages (Utilities|Struct|BreakTrainSpline _array_element))
      (Transformation|SetWorldLocationAndRotation _array_element_2 (Spline|GetLocationatDistanceAlongSpline (.spline (Utilities|Struct|BreakTrainSpline _array_element)) (|(((splinePosition+(splineLength-(1200*index)))+0.010000)%splineLength) (Math|Interpolation|Ease "EaseInOut" (|(((((max((time-delay),0))*{47F61FAE-4EFC-818D-3832-1E9862E6ED00})*55.555555)/splineLength)%1) (Utilities|Time|GetGameTimeinSeconds) (Spline|GetSplineLength (.spline (Utilities|Struct|BreakTrainSpline _array_element))) (.delay (Utilities|Struct|BreakTrainSpline _array_element))) 0.0 (Spline|GetSplineLength (.spline (Utilities|Struct|BreakTrainSpline _array_element))) 1.8) (Spline|GetSplineLength (.spline (Utilities|Struct|BreakTrainSpline _array_element))) _array_index) "World") (Math|Rotator|CombineRotators (Spline|GetRotationatDistanceAlongSpline (.spline (Utilities|Struct|BreakTrainSpline _array_element)) (|(((splinePosition+(splineLength-(1200*index)))+0.010000)%splineLength) (Math|Interpolation|Ease "EaseInOut" (|(((((max((time-delay),0))*{47F61FAE-4EFC-818D-3832-1E9862E6ED00})*55.555555)/splineLength)%1) (Utilities|Time|GetGameTimeinSeconds) (Spline|GetSplineLength (.spline (Utilities|Struct|BreakTrainSpline _array_element))) (.delay (Utilities|Struct|BreakTrainSpline _array_element))) 0.0 (Spline|GetSplineLength (.spline (Utilities|Struct|BreakTrainSpline _array_element))) 1.8) (Spline|GetSplineLength (.spline (Utilities|Struct|BreakTrainSpline _array_element))) _array_index) "World") (Utilities|Array|Get(acopy) (.flips (Utilities|Struct|BreakTrainSpline _array_element)) _array_index)) false false))))

(fn ConstructionScript
  (Utilities|FlowControl|Sequence
    (:then_0
      ;[1 1 1] rail splines map
      (Variables|Default|SetrailSplineBlueprints (Utilities|Map|MakeMap "I" (Variables|Default|Getstraight-rail_spline) "L" (Variables|Default|Getcurved-rail-L_spline) "/" (Variables|Default|Getskewed-rail_spline) "R" (Variables|Default|Getcurved-rail-R_spline))))
    (:then_1
      (bind _asjson_loader (Utilities|Casting|CastTojson-loader (Actor|GetParentActor)))
      (for _array_element (Variables|/Game/MyStuff/BLUEPRINTS/json-loader/json-loader.json-loader_C|GettrainPaths _asjson_loader)
        (Utilities|FlowControl|Sequence
          (:then_0
            (bind _returnvalue (AddComponent|AddSplineComponent false))
            (Spline|ClearSplinePoints _returnvalue true)
            (Development|SetHiddeninGame _returnvalue false false)
            (bind (_item_1 _item_2 _index_1) (Utilities|ForEachPairwise (.path (Utilities|Struct|BreakTrainPath _array_element)))
              (:Loop%20body
                ;[1 1 1] Create spline
                (bind (_position _tangent) (CallFunction|GetRailSplinePoint _item_1 false))
                (bind (_position_2 _tangent_2) (CallFunction|GetRailSplinePoint _item_2 true))
                (Spline|AddSplinePoint _returnvalue (Math|Vector|SelectVector _position _position_2 (>= _index_1 0)) "Local" true)
                (Spline|SetTangentsatSplinePoint _returnvalue (+ _index_1 1) (Math|Vector|SelectVector _tangent "0, 0, 0" (>= _index_1 0)) _tangent_2 "Local" true))))
          (:then_1
            ;[1 1 1] Close spline if ends are close enough
            (if (< (Class|KismetMathLibrary|VectorDistanceSquared (Spline|GetLocationatSplinePoint _returnvalue 0 "Local") (Spline|GetLocationatSplinePoint _returnvalue (- (Spline|GetNumberOfSplinePoints _returnvalue) 1) "Local")) 1.61e+04)
              (Spline|SetClosedLoop _returnvalue true true)))
          (:then_2
            ;[1 1 1] Place carriages on spline
            (bind _arrayout (Utilities|SetTempArray (Utilities|Array|MakeArray))
              (:ExecOut
                (bind _arrayout_2 (Utilities|SetTempArray (Utilities|Array|MakeArray))
                  (:ExecOut
                    (for (_array_element_2 _array_index) (.carriges (Utilities|Struct|BreakTrainPath _array_element))
                      (bind _returnvalue_2 (AddComponent|AddChildActorComponent false))
                      (Utilities|Array|Add _arrayout_2 _returnvalue_2)
                      (ChildActorComponent|SetChildActorClass _returnvalue_2 (.Value (Utilities|Map|Find (Variables|Default|GetcarriageBlueprints) (Variables|/Game/MyStuff/BLUEPRINTS/json-loader/ExportedEntity.ExportedEntity_C|Getname _array_element_2))))
                      (Utilities|Array|Add _arrayout (Math|Rotator|MakeRotator 0.0 0.0 (select (Variables|/Game/MyStuff/BLUEPRINTS/json-loader/ExportedEntity.ExportedEntity_C|Getback_mover _array_element_2) 1.8e+02 0.0)))
                      (Transformation|SetWorldLocationAndRotation _returnvalue_2 (Spline|GetLocationatDistanceAlongSpline _returnvalue (|(((splineLength-(carriageIndex*1200))+0.010000)%splineLength) (Spline|GetSplineLength _returnvalue) _array_index) "World") (Math|Rotator|CombineRotators (Spline|GetRotationatDistanceAlongSpline _returnvalue (|(((splineLength-(carriageIndex*1200))+0.010000)%splineLength) (Spline|GetSplineLength _returnvalue) _array_index) "World") (Math|Rotator|MakeRotator 0.0 0.0 (select (Variables|/Game/MyStuff/BLUEPRINTS/json-loader/ExportedEntity.ExportedEntity_C|Getback_mover _array_element_2) 1.8e+02 0.0))) false true)
                      (Utilities|Array|Add (Variables|Default|GettrainSplines) (Utilities|Struct|MakeTrainSpline _returnvalue _arrayout_2 _arrayout (Math|Random|RandomFloatinRange 0.0 5.0))))))))))))))

(fn GetRailSplinePoint
  (params (rail :type Train%20Path%20Segment%20Structure%20%28by%20ref%29) (isRailStart :type Boolean))
  (bind (_entity _invert_spline) (Utilities|Struct|BreakTrainPathSegment rail))
  (bind _railsplineblueprints (Variables|Default|GetrailSplineBlueprints))
  (bind _returnvalue (!= isRailStart _invert_spline))
  (bind _variant (Variables|/Game/MyStuff/BLUEPRINTS/json-loader/ExportedEntity.ExportedEntity_C|Getvariant _entity))
  (bind _direction (Variables|/Game/MyStuff/BLUEPRINTS/json-loader/ExportedEntity.ExportedEntity_C|Getdirection _entity))
  (bind _returnvalue_2 (Math|Integer|SelectInt 0 1 _returnvalue))
  (bind _value (Utilities|Map|Find _railsplineblueprints _variant))
  (bind _returnvalue_3 (|(direction*45.000000) _direction))
  (bind _returnvalue_4 (Math|Rotator|MakeRotator 0.0 0.0 _returnvalue_3))
  (bind _returnvalue_5 (Spline|GetArriveTangentatSplinePoint _value _returnvalue_2 "Local"))
  (bind _returnvalue_6 (Spline|GetLeaveTangentatSplinePoint _value _returnvalue_2 "Local"))
  (bind _returnvalue_7 (Math|Vector|SelectVector _returnvalue_6 _returnvalue_5 _returnvalue))
  (return (+ (Math|Vector|RotateVector (Spline|GetLocationatSplinePoint _value _returnvalue_2 "Local") _returnvalue_4) (Variables|/Game/MyStuff/BLUEPRINTS/json-loader/ExportedEntity.ExportedEntity_C|Getlocation _entity)) (Math|Vector|RotateVector (Math|Vector|SelectVector (Math|Vector|RotateVector _returnvalue_7 "0.000000,180.000000,0.000000") _returnvalue_7 _invert_spline) _returnvalue_4)))