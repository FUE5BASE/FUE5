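; Ground actor that fakes an infinite floor with a single, hugely scaled plane.
; The construction script creates a dynamic instance of the chosen surface material, feeds it the U and V tiling variables, and applies it to the plane.
; It also pins the plane just below the world origin in world space, regardless of actor placement.
; The event graph is empty, so all setup happens at construction.
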(event EventBeginPlay)

(event Collision|EventActorBeginOverlap
  (params (OtherActor :type Actor%20Object%20Reference)))

(event EventTick
  (params (DeltaSeconds :type Float%20%28single-precision%29)))

(fn ConstructionScript
  (bind _plane (Variables|Default|GetPlane))
  ;[1 1 1] make plane
  (bind _returnvalue (Rendering|Material|CreateDynamicMaterialInstance (Variables|Default|Getsurface-material) "" "None" :!class /Script/Engine.KismetMaterialLibrary))
  (Rendering|Material|SetScalarParameterValue _returnvalue "UTiling" (Math|Conversions|ToFloat(Integer) (Variables|Default|GetUTiling)) :!class /Script/Engine.MaterialInstanceDynamic)
  (Rendering|Material|SetScalarParameterValue _returnvalue "VTiling" (Math|Conversions|ToFloat(Integer) (Variables|Default|GetVTiling)) :!class /Script/Engine.MaterialInstanceDynamic)
  (Rendering|Material|SetMaterial _plane 0 _returnvalue)
  (Transformation|SetWorldLocation _plane "0.000000,0.000000,-1.000000" false false)
  (Transformation|SetRelativeScale3D _plane "1000.000000,1000.000000,1000.000000"))