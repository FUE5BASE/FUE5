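; Belt system that builds two-lane conveyor belts from exported entity JSON and animates items along them.
; The construction script stitches splines for each belt path from rotated straight, left and right template shapes.
; It fills both lanes with random child-actor items from that lane's list, zero-scaling some by a fullness percentage.
; Tick loops items along splines by game time, using cumulative end indices into one flat item array.
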(event EventTick
  (params (DeltaSeconds :type Float%20%28single-precision%29))
  (bind _item_ends (Variables|Default|Getitem-ends))
  (for (_array_element _array_index) _item_ends
    (for _index (range (select (> _array_index 0) (Utilities|Array|Get(acopy) _item_ends (- _array_index 1)) (Class|KismetSystemLibrary|MakeLiteralInteger)) (- _array_element 1))
      (Utilities|FlowControl|Sequence
        (:then_0
          (Transformation|SetWorldLocation (Utilities|Array|Get(acopy) (Variables|Default|Getitems-on-belts) _index) (.Location (Math|Transform|BreakTransform (Math|Transform|ComposeTransforms (Math|Transform|MakeTransform (Math|Vector|MakeVector 0.0 (* (Math|Float|SelectFloat 1.0 -1.0 (>= (- _index (select (> _array_index 0) (Utilities|Array|Get(acopy) _item_ends (- _array_index 1)) (Class|KismetSystemLibrary|MakeLiteralInteger))) (/ (- _array_element (select (> _array_index 0) (Utilities|Array|Get(acopy) _item_ends (- _array_index 1)) (Class|KismetSystemLibrary|MakeLiteralInteger))) 2))) (Variables|Default|Getlane-spacing)) 0.0)) (Spline|GetTransformatDistanceAlongSpline (Utilities|Array|Get(acopy) (Variables|Default|Getsplines) _array_index) (Math|Float|%(Float) (+ (* 1.7e+02 (Utilities|Time|GetGameTimeinSeconds)) (* (Math|Integer|%(Integer) (- _index (select (> _array_index 0) (Utilities|Array|Get(acopy) _item_ends (- _array_index 1)) (Class|KismetSystemLibrary|MakeLiteralInteger))) (/ (- _array_element (select (> _array_index 0) (Utilities|Array|Get(acopy) _item_ends (- _array_index 1)) (Class|KismetSystemLibrary|MakeLiteralInteger))) 2)) (Variables|Default|Getitem-spacing))) (Spline|GetSplineLength (Utilities|Array|Get(acopy) (Variables|Default|Getsplines) _array_index))) "World" false)))) false false)
          (Transformation|SetWorldRotation (Utilities|Array|Get(acopy) (Variables|Default|Getitems-on-belts) _index) (.Rotation (Math|Transform|BreakTransform (Math|Transform|ComposeTransforms (Math|Transform|MakeTransform (Math|Vector|MakeVector 0.0 (* (Math|Float|SelectFloat 1.0 -1.0 (>= (- _index (select (> _array_index 0) (Utilities|Array|Get(acopy) _item_ends (- _array_index 1)) (Class|KismetSystemLibrary|MakeLiteralInteger))) (/ (- _array_element (select (> _array_index 0) (Utilities|Array|Get(acopy) _item_ends (- _array_index 1)) (Class|KismetSystemLibrary|MakeLiteralInteger))) 2))) (Variables|Default|Getlane-spacing)) 0.0)) (Spline|GetTransformatDistanceAlongSpline (Utilities|Array|Get(acopy) (Variables|Default|Getsplines) _array_index) (Math|Float|%(Float) (+ (* 1.7e+02 (Utilities|Time|GetGameTimeinSeconds)) (* (Math|Integer|%(Integer) (- _index (select (> _array_index 0) (Utilities|Array|Get(acopy) _item_ends (- _array_index 1)) (Class|KismetSystemLibrary|MakeLiteralInteger))) (/ (- _array_element (select (> _array_index 0) (Utilities|Array|Get(acopy) _item_ends (- _array_index 1)) (Class|KismetSystemLibrary|MakeLiteralInteger))) 2)) (Variables|Default|Getitem-spacing))) (Spline|GetSplineLength (Utilities|Array|Get(acopy) (Variables|Default|Getsplines) _array_index))) "World" false)))) false false))))))

(fn ConstructionScript
  (bind _returnvalue (Class|BlueprintPathsLibrary|GetProjectFilePath))
  (bind _self_reference (Variables|Default|Getself-reference))
  ;[1 1 1] json parser
  (Utilities|FlowControl|Sequence
    (:then_0
      ;[1 1 1] make spline map for each belt shape
      (Variables|Default|Setbelt-splines-map (Utilities|Map|MakeMap "I" (Variables|Default|Getbelt-I_spline) "L" (Variables|Default|Getbelt-L_spline) "R" (Variables|Default|Getbelt-R_spline))))
    (:then_1
      (bind _outjsonobject (Class|JsonBlueprintFunctionLibrary|FromFile (Utilities|Struct|MakeFilePath (Utilities|String|SelectString (Class|KismetSystemLibrary|ConverttoAbsolutePath (Class|BlueprintPathsLibrary|Combine (Utilities|Array|MakeArray (Utilities|String|LeftChop _returnvalue (Utilities|String|Len (Class|BlueprintPathsLibrary|GetCleanFilename _returnvalue))) "Content" (Utilities|String|RightChop (Utilities|String|LeftChop (Class|KismetSystemLibrary|GetPathName _self_reference) (|((x*2)+1) (Utilities|String|Len (Utilities|GetObjectName _self_reference)))) 6) "exported-entities.json"))) (Class|BlueprintPathsLibrary|Combine (Utilities|Array|MakeArray (Class|KismetSystemLibrary|GetProjectDirectory) "Content" "MyStuff" "JSON" "exported-entities.json")) (Variables|Default|Getlocal-json)))))
      (bind _outvalue (|GetJsonField _outjsonobject "entities"))
      (bind _outvalue_2 (|GetJsonField _outjsonobject "belt_paths"))
      (for _array_element _outvalue_2
        ;[1 1 1] make each spline
        (bind _returnvalue_2 (AddComponent|AddSplineComponent false))
        (Spline|ClearSplinePoints _returnvalue_2 true)
        (Rendering|SetVisibility _returnvalue_2 false false)
        (Spline|SetClosedLoop _returnvalue_2 false true)
        (Development|SetHiddeninGame _returnvalue_2 true false)
        (Utilities|Array|Add (Variables|Default|Getsplines) _returnvalue_2)
        (bind _outvalue_3 (|GetJsonField _array_element "path"))
        (bind _outvalue_4 (|GetJsonField _array_element "items_lane_1"))
        (bind _outvalue_5 (|GetJsonField _array_element "items_lane_2"))
        (for _index (range 0 (Utilities|Array|Length _outvalue_3))
          (bind (_position _tangent) (CallFunction|Get-spline-point (Utilities|Array|Get(acopy) _outvalue (Utilities|Array|Get(acopy) _outvalue_3 (+ _index -1))) false))
          (bind (_position_2 _tangent_2) (CallFunction|Get-spline-point (Utilities|Array|Get(acopy) _outvalue (Utilities|Array|Get(acopy) _outvalue_3 _index)) true))
          (Spline|AddSplinePoint _returnvalue_2 (+ (Math|Vector|SelectVector _position_2 _position (== _index 0)) "0.000000,0.000000,50.000000") "Local" true)
          (Spline|SetTangentsatSplinePoint _returnvalue_2 _index _tangent _tangent_2 "Local" true))
        ;[1 1 1] make items
        ;;[1 1 1] reset for each spline
        (Utilities|FlowControl|Sequence
          (:then_0
            (goto _label_2 Reset))
          (:then_1
            (Variables|Default|Setlane-switcher 1)
            (for _index_2 (range 0 (Math|Float|Truncate (/ (Spline|GetSplineLength _returnvalue_2) (Variables|Default|Getitem-spacing)))) :!label _label
              (bind _returnvalue_3 (AddComponent|AddChildActorComponent false))
              (Utilities|FlowControl|Sequence
                (:then_0
                  (Utilities|Array|Add (Variables|Default|Getitems-on-belts) _returnvalue_3))
                (:then_1
                  (ChildActorComponent|SetChildActorClass _returnvalue_3 (.Value (Utilities|Map|Find (Variables|Default|Getitem-list) (select (== (Variables|Default|Getlane-switcher) 1) (.OutItem (Utilities|Array|Random _outvalue_5)) (.OutItem (Utilities|Array|Random _outvalue_4))))))
                  (Transformation|SetRelativeTransform _returnvalue_3 (Math|Transform|MakeTransform (+ (.Location (Math|Transform|BreakTransform (Math|Transform|ComposeTransforms (Math|Transform|MakeTransform (Math|Vector|MakeVector 0.0 (Math|Conversions|ToFloat(Integer) (* (Variables|Default|Getlane-spacing) (Variables|Default|Getlane-switcher))) 0.0)) (Spline|GetTransformatDistanceAlongSpline _returnvalue_2 (Math|Conversions|ToFloat(Integer) (* _index_2 (Variables|Default|Getitem-spacing))) "Local" false)))) "") (Math|Rotator|CombineRotators "0.000000,0.000000,4.000000" "0, 0, 0")) false false)
                  (Math|Integer|CompareInt (Math|Random|RandomIntegerinRange 1 100) (Variables|Default|Getbelt-fullness)
                    (:>
                      (Transformation|SetWorldScale3D _returnvalue_3 "0, 0, 0"))))))
            (Variables|Default|Setlane-switcher -1)
            (Utilities|FlowControl|DoOnce false :!label _label_2
              (:Completed
                (goto _label))))
          (:then_2
            ;[1 1 1] set items ends
            (Utilities|Array|Add (Variables|Default|Getitem-ends) (Utilities|Array|Length (Variables|Default|Getitems-on-belts)))))))))

(fn Get-spline-point
  (params (rail :type Json%20Object%20Wrapper%20Structure%20%28by%20ref%29) (isRailStart :type Boolean))
  (bind _returnvalue (Math|Integer|SelectInt 0 1 isRailStart))
  (bind _outvalue (|GetJsonField rail "variant"))
  (bind _outvalue_2 (|GetJsonField rail "x"))
  (bind _outvalue_3 (|GetJsonField rail "y"))
  (bind _outvalue_4 (|GetJsonField rail "direction"))
  (return (+ (Math|Vector|RotateVector (Spline|GetLocationatSplinePoint (.Value (Utilities|Map|Find (Variables|Default|Getbelt-splines-map) _outvalue)) _returnvalue "Local") (Math|Rotator|MakeRotator 0.0 0.0 (Math|Conversions|ToFloat(Integer) (* _outvalue_4 45)))) (* (Math|Vector|MakeVector _outvalue_2 _outvalue_3 0.0) "200.000000,200.000000,0.000000")) (Math|Vector|RotateVector (select isRailStart (Spline|GetLeaveTangentatSplinePoint (.Value (Utilities|Map|Find (Variables|Default|Getbelt-splines-map) _outvalue)) _returnvalue "Local") (Spline|GetArriveTangentatSplinePoint (.Value (Utilities|Map|Find (Variables|Default|Getbelt-splines-map) _outvalue)) _returnvalue "Local")) (Math|Rotator|MakeRotator 0.0 0.0 (Math|Conversions|ToFloat(Integer) (* _outvalue_4 45))))))