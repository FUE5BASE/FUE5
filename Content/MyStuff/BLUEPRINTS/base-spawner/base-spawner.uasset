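; Base spawner that builds a base layout from exported-entities JSON (local or global file) in its construction script.
; Entity names resolve through class maps to child actors placed on a scaled grid, with variants set via _HasVariants; names in the Missing map become cubes.
; The largest coordinates scale the level's Landscape and a tiled-material ground mesh.
; Wire connections become child actors aimed and stretched between endpoints.
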(fn ConstructionScript
  (bind _returnvalue (Class|BlueprintPathsLibrary|GetProjectFilePath))
  (bind _returnvalue_2 (Math|Float|MakeLiteralFloat 1.0))
  (bind _returnvalue_3 (Math|Float|MakeLiteralFloat 0.12))
  (bind _returnvalue_4 (Math|Float|MakeLiteralFloat 3.573))
  (bind _static (Variables|Default|Getstatic))
  (bind _self_reference (Variables|Default|Getself-reference))
  ;[1 1 1] json parser
  (Utilities|FlowControl|Sequence
    (:then_0
      (bind _outjsonobject (Class|JsonBlueprintFunctionLibrary|FromFile (Utilities|Struct|MakeFilePath (Utilities|String|SelectString (Class|KismetSystemLibrary|ConverttoAbsolutePath (Class|BlueprintPathsLibrary|Combine (Utilities|Array|MakeArray (Utilities|String|LeftChop _returnvalue (Utilities|String|Len (Class|BlueprintPathsLibrary|GetCleanFilename _returnvalue))) "Content" (Utilities|String|RightChop (Utilities|String|LeftChop (Class|KismetSystemLibrary|GetPathName _self_reference) (|((x*2)+1) (Utilities|String|Len (Utilities|GetObjectName _self_reference)))) 6) "exported-entities.json"))) (Class|BlueprintPathsLibrary|Combine (Utilities|Array|MakeArray (Class|KismetSystemLibrary|GetProjectDirectory) "Content" "MyStuff" "JSON" "exported-entities.json")) (Variables|Default|Getlocal-json)))))
      (bind _outvalue (|GetJsonField _outjsonobject "entities"))
      (for _array_element _outvalue
        (Utilities|FlowControl|Sequence
          (:then_0
            (bind _outvalue_2 (|GetJsonField _array_element "name"))
            (bind _outvalue_3 (|GetJsonField _array_element "variant"))
            ;[1 1 1] coordinate translate
            (bind _outvalue_4 (|GetJsonField _array_element "x"))
            (bind _outvalue_5 (|GetJsonField _array_element "y"))
            (bind _outvalue_6 (|GetJsonField _array_element "direction"))
            (bind _outvalue_7 (|GetJsonField _array_element "width"))
            (bind _outvalue_8 (|GetJsonField _array_element "height"))
            ;[1 1 1] choose entity and spawn
            (bind _returnvalue_5 (AddComponent|AddChildActorComponent false (Math|Transform|MakeTransform (* (Math|Vector|MakeVector _outvalue_4 _outvalue_5 0.0) "200.000000,200.000000,200.000000") (* (Math|Rotator|MakeRotator 0.0 0.0 _outvalue_6) 45.0) (Math|Vector|MakeVector 1.0 1.0 1.0))))
            (if (.ReturnValue (Utilities|Map|Find (Variables|Default|Getvariants) _outvalue_2))
              (ChildActorComponent|SetChildActorClass _returnvalue_5 (.Value (Utilities|Map|Find (Variables|Default|Getvariants) _outvalue_2)))
              (bind _as_has_variants (Utilities|Casting|CastTo_HasVariants (Variables|/Script/Engine.ChildActorComponent|GetChildActor _returnvalue_5) :!label _label))
              (Default|SetVariant _as_has_variants _outvalue_3)
              (elif (.ReturnValue (Utilities|Map|Find (Variables|Default|Getstructures) _outvalue_2))
                (ChildActorComponent|SetChildActorClass _returnvalue_5 (.Value (Utilities|Map|Find (Variables|Default|Getstructures) _outvalue_2)))
                (goto _label)
                (elif (.ReturnValue (Utilities|Map|Find (Variables|Default|Getpower) _outvalue_2))
                  (ChildActorComponent|SetChildActorClass _returnvalue_5 (.Value (Utilities|Map|Find (Variables|Default|Getpower) _outvalue_2)))
                  (goto _label)
                  (elif (.ReturnValue (Utilities|Map|Find (Variables|Default|Getfoliage) _outvalue_2))
                    (ChildActorComponent|SetChildActorClass _returnvalue_5 (.Value (Utilities|Map|Find (Variables|Default|Getfoliage) _outvalue_2)))
                    (goto _label)
                    (elif (.ReturnValue (Utilities|Map|Find (Variables|Default|Getmissing) _outvalue_2))
                      (bind _returnvalue_6 (AddComponent|AddStaticMeshComponent false (Math|Transform|MakeTransform (* (Math|Vector|MakeVector _outvalue_4 _outvalue_5 0.0) "200.000000,200.000000,200.000000") (* (Math|Rotator|MakeRotator 0.0 0.0 _outvalue_6) 45.0) (* (Math|Vector|MakeVector _outvalue_7 _outvalue_8 1.0) "2.000000,2.000000,2.000000"))))
                      (Components|StaticMesh|SetStaticMesh _returnvalue_6 "/Game/StarterContent/Shapes/Shape_Cube.Shape_Cube")))))))
          (:then_1
            ;[0.2415 0.5417 0.1487] ground spawner
            ;;[1 1 1] coordinate translate
            (bind _outvalue_9 (|GetJsonField _array_element "x"))
            (Utilities|FlowControl|Sequence
              (:then_1
                (Math|Float|CompareFloat _outvalue_9 (Variables|Default|Getx_end)
                  (:>
                    (Variables|Default|Setx_end _outvalue_9))))
              (:then_2
                (bind _outvalue_10 (|GetJsonField _array_element "y"))
                (Utilities|FlowControl|Sequence
                  (:then_1
                    (Math|Float|CompareFloat _outvalue_10 (Variables|Default|Gety_end)
                      (:>
                        (Variables|Default|Sety_end _outvalue_10))))))))))
      ;;[1 1 1] landscape scale
      (bind _outactors (Actor|GetAllActorsOfClass "/Script/Landscape.Landscape"))
      (Transformation|SetActorScale3D (Utilities|Array|Get(acopy) _outactors) (Math|Vector|MakeVector (* (Variables|Default|Getx_end) _returnvalue_4) (* (Variables|Default|Gety_end) _returnvalue_4) (* (Variables|Default|Gety_end) _returnvalue_4)))
      ;;[1 1 1] make plane
      (bind _returnvalue_7 (Rendering|Material|CreateDynamicMaterialInstance (Variables|Default|Getground-material) "" "None" :!class /Script/Engine.KismetMaterialLibrary))
      (Rendering|Material|SetScalarParameterValue _returnvalue_7 "UTiling" (* (Variables|Default|Getx_end) _returnvalue_3) :!class /Script/Engine.MaterialInstanceDynamic)
      (Rendering|Material|SetScalarParameterValue _returnvalue_7 "VTiling" (* (Variables|Default|Gety_end) _returnvalue_3) :!class /Script/Engine.MaterialInstanceDynamic)
      (Rendering|Material|SetMaterial _static 0 _returnvalue_7)
      (Transformation|SetRelativeScale3D _static (Math|Vector|MakeVector (* (Variables|Default|Getx_end) _returnvalue_2) (* (Variables|Default|Gety_end) _returnvalue_2) 1.0)))
    (:then_1
      ;[1 1 1] wires
      (bind _outvalue_11 (|GetJsonField _outjsonobject "wire_connections"))
      (for _array_element_2 _outvalue_11
        (bind _outvalue_12 (|GetJsonField _array_element_2 "start"))
        (bind _outvalue_13 (|GetJsonField _array_element_2 "target"))
        (bind _outvalue_14 (|GetJsonField _outvalue_12 "x"))
        (bind _outvalue_15 (|GetJsonField _outvalue_12 "y"))
        (bind _outvalue_16 (|GetJsonField _outvalue_12 "z"))
        (bind _outvalue_17 (|GetJsonField _outvalue_13 "x"))
        (bind _outvalue_18 (|GetJsonField _outvalue_13 "y"))
        (bind _outvalue_19 (|GetJsonField _outvalue_13 "z"))
        (bind _returnvalue_8 (AddComponent|AddChildActorComponent false (Math|Conversions|ToTransform(Vector) (* (Math|Vector|MakeVector _outvalue_14 _outvalue_15 _outvalue_16) "200.000000,200.000000,200.000000"))))
        (Transformation|SetRelativeRotation _returnvalue_8 (Math|Rotator|FindLookatRotation (* (Math|Vector|MakeVector _outvalue_14 _outvalue_15 _outvalue_16) "200.000000,200.000000,200.000000") (* (Math|Vector|MakeVector _outvalue_17 _outvalue_18 _outvalue_19) "200.000000,200.000000,200.000000")) false false)
        (Transformation|SetWorldScale3D _returnvalue_8 (Math|Vector|MakeVector (/ (Math|Vector|VectorLength (- (* (Math|Vector|MakeVector _outvalue_14 _outvalue_15 _outvalue_16) "200.000000,200.000000,200.000000") (* (Math|Vector|MakeVector _outvalue_17 _outvalue_18 _outvalue_19) "200.000000,200.000000,200.000000"))) 4e+02) 1.0 1.0))))))

(fn NewFunction
  (params (Selection :type String))
  (switch string Selection))