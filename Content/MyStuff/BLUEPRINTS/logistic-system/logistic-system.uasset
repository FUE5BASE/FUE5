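; Logistic system actor that builds roboports with robots from an exported entities JSON when its construction script runs.
; It reads either a JSON beside its own asset path or a global one, selected by the Localjson flag.
; Chest indices in the logistic systems resolve to scaled entity positions, which are collected and passed to each roboport spawned as a child actor component.
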(event EventBeginPlay)

(event Collision|EventActorBeginOverlap
  (params (OtherActor :type Actor%20Object%20Reference)))

(event EventTick
  (params (DeltaSeconds :type Float%20%28single-precision%29)))

(fn ConstructionScript
  (bind _returnvalue (Class|BlueprintPathsLibrary|GetProjectFilePath))
  (bind _self_reference (Variables|Default|Getself-reference))
  (bind _outjsonobject (Class|JsonBlueprintFunctionLibrary|FromFile (Utilities|Struct|MakeFilePath (Utilities|String|SelectString (Class|KismetSystemLibrary|ConverttoAbsolutePath (Class|BlueprintPathsLibrary|Combine (Utilities|Array|MakeArray (Utilities|String|LeftChop _returnvalue (Utilities|String|Len (Class|BlueprintPathsLibrary|GetCleanFilename _returnvalue))) "Content" (Utilities|String|RightChop (Utilities|String|LeftChop (Class|KismetSystemLibrary|GetPathName _self_reference) (|((x*2)+1) (Utilities|String|Len (Utilities|GetObjectName _self_reference)))) 6) "exported-entities.json"))) (Class|BlueprintPathsLibrary|Combine (Utilities|Array|MakeArray (Class|KismetSystemLibrary|GetProjectDirectory) "Content" "MyStuff" "JSON" "exported-entities.json")) (Variables|Default|Getlocal-json)))))
  (bind _outvalue (|GetJsonField _outjsonobject "logistic_systems"))
  (bind _outvalue_2 (|GetJsonField _outjsonobject "entities"))
  (for _array_element _outvalue
    (bind _outvalue_3 (|GetJsonField _array_element "chests"))
    (for _array_element_2 _outvalue_3
      (bind _outvalue_4 (|GetJsonField (Utilities|Array|Get(acopy) _outvalue_2 _array_element_2) "x"))
      (bind _outvalue_5 (|GetJsonField (Utilities|Array|Get(acopy) _outvalue_2 _array_element_2) "y"))
      (Utilities|Array|Add (Variables|Default|GetchestPositions) (* (Math|Vector|MakeVector _outvalue_4 _outvalue_5 0.0) "200.000000,200.000000,200.000000"))))
  (bind _outvalue_6 (|GetJsonField _array_element "roboports"))
  (for _array_element_3 _outvalue_6
    (bind _outvalue_7 (|GetJsonField (Utilities|Array|Get(acopy) _outvalue_2 _array_element_3) "x"))
    (bind _outvalue_8 (|GetJsonField (Utilities|Array|Get(acopy) _outvalue_2 _array_element_3) "y"))
    (bind _returnvalue_2 (AddComponent|AddChildActorComponent false (Math|Conversions|ToTransform(Vector) (* (Math|Vector|MakeVector _outvalue_7 _outvalue_8 0.0) "200.000000,200.000000,200.000000"))))
    (ChildActorComponent|SetChildActorClass _returnvalue_2 "/Game/MyStuff/ENTITIES/STRUCTURES/roboport/bp/roboport_withRobots.roboport_withRobots_C")
    (bind _asroboport_with_robots (Utilities|Casting|CastToroboport_withRobots (Variables|/Script/Engine.ChildActorComponent|GetChildActor _returnvalue_2)))
    (Default|SetChestPositions _asroboport_with_robots (Variables|Default|GetchestPositions)))
  (Utilities|Array|Clear (Variables|Default|GetchestPositions)))